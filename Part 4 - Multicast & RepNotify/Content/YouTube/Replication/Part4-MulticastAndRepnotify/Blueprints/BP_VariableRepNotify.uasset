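; BP_VariableRepNotify is a replication demo that shows a RepNotify variable driving a randomly changing emissive color.
; On BeginPlay, only the authority starts a looping one-second timer that sets Variable to a color built from a random unit vector.
; OnRep_Variable applies that value to the material's EmissiveColor parameter.
; The construction script calls its parent, then raises the material's emissive strength.
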(event Custom|Update
  (Variables|Default|SetVariable (Math|Conversions|ToLinearColor(Vector) (Math|Random|RandomUnitVector))))

(event EventBeginPlay
  (Networking|SwitchHasAuthority
    (:Authority
      (Utilities|Time|SetTimerbyEvent (delegate Custom|Update) 1.0 true))))

(fn ConstructionScript
  (|CallParentFunction)
  (Rendering|Material|SetScalarParameterValue (Variables|Default|GetMaterial) "EmissiveStrength" 1e+01 :!class /Script/Engine.MaterialInstanceDynamic))

(fn OnRepVariable
  (Rendering|Material|SetVectorParameterValue (Variables|Default|GetMaterial) "EmissiveColor" (Variables|Default|GetVariable) :!class /Script/Engine.MaterialInstanceDynamic))