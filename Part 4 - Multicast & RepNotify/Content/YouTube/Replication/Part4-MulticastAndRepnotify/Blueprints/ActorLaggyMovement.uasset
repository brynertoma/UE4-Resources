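; Replication tutorial actor that moves an emissive-black sphere around a spline at ever-increasing speed.
; Move lerps the sphere to the spline's last point, toggles every PP_Player's camera, then loops a timeline along the spline's distance.
; Each lap raises the play rate, and past a threshold every lap also shakes all players.
; BeginPlay looks up BP_GoodSky actors, setting a retry timer until exactly two exist.
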(event Custom|Move
  (bind _spline (Variables|Default|GetSpline))
  (bind _spline_2 (Variables|Default|GetSpline))
  (bind _spline_3 (Variables|/Game/YouTube/Replication/Part4-MulticastAndRepnotify/Blueprints/BP_Spline.BP_Spline_C|GetSpline _spline_2))
  (bind _spline_4 (Variables|/Game/YouTube/Replication/Part4-MulticastAndRepnotify/Blueprints/BP_Spline.BP_Spline_C|GetSpline _spline))
  (Variables|Default|SetSplineStart (Spline|GetLocationatSplinePoint _spline_3 (- (Spline|GetNumberOfSplinePoints _spline_3) 1) "World"))
  (Components|Timeline|SetPlayRate (Variables|Default|GetStartTimeline) 0.5)
  (bind _alpha (Timeline|StartTimeline PlayFromStart)
    (:Update
      (Transformation|SetRelativeLocation (Variables|Default|GetSphere) (Math|Vector|Lerp(Vector) "0,0.000000,1000.000000" (Variables|Default|GetSplineStart) _alpha) false false))
    (:Finished
      (CallFunction|MoveCamera)
      (Components|Timeline|SetPlayRate (Variables|Default|GetMoveTimeline) (Variables|Default|GetPlayRate))
      (Variables|Default|SetSplineLength (- (Spline|GetDistanceAlongSplineatSplinePoint _spline_4 (- (Spline|GetNumberOfSplinePoints (Variables|/Game/YouTube/Replication/Part4-MulticastAndRepnotify/Blueprints/BP_Spline.BP_Spline_C|GetSpline (Variables|Default|GetSpline))) 1)) (Spline|GetDistanceAlongSplineatSplinePoint _spline_4 0)))
      (bind _alpha_2 (Timeline|MoveTimeline PlayFromStart)
        (:Update
          (Transformation|SetRelativeLocation (Variables|Default|GetSphere) (Spline|GetLocationatDistanceAlongSpline (Variables|/Game/YouTube/Replication/Part4-MulticastAndRepnotify/Blueprints/BP_Spline.BP_Spline_C|GetSpline (Variables|Default|GetSpline)) (Math|Float|Lerp 0.0 (Variables|Default|GetSplineLength) _alpha_2) "World") false false))
        (:Finished
          (bind _output_get (Variables|Default|SetPlayRate (+ (Variables|Default|GetPlayRate) 0.02)))
          (Components|Timeline|SetPlayRate (Variables|Default|GetMoveTimeline) _output_get)
          (if (>= _output_get 3.0)
            (CallFunction|Shake)
            (Timeline|MoveTimeline PlayFromStart)
            (else
              (Timeline|MoveTimeline PlayFromStart))))))))

(event Custom|MoveCamera
  (bind _outactors (Actor|GetAllActorsOfClass "/Game/YouTube/Replication/Part4-MulticastAndRepnotify/PP_Player.PP_Player_C"))
  (for _array_element _outactors
    (Default|ToggleCamera _array_element)))

(event Custom|Retry
  (bind _outactors (Actor|GetAllActorsOfClass "/Game/YouTube/Assets/3rdParty/GoodSky/Blueprint/BP_GoodSky.BP_GoodSky_C"))
  (bind _output_get (Variables|Default|SetSky _outactors))
  (if (not (== (Utilities|Array|Length _output_get) 2))
    (Utilities|Time|SetTimerbyEvent (EventDispatchers|CreateEvent :!event Custom|Retry) 1.0)))

(event Custom|Shake
  (bind _outactors (Actor|GetAllActorsOfClass "/Game/YouTube/Replication/Part4-MulticastAndRepnotify/PP_Player.PP_Player_C"))
  (for _array_element _outactors
    (Default|ShakeyWakey _array_element)))

(event EventBeginPlay
  (bind _outactors (Actor|GetAllActorsOfClass "/Game/YouTube/Assets/3rdParty/GoodSky/Blueprint/BP_GoodSky.BP_GoodSky_C"))
  (bind _output_get (Variables|Default|SetSky _outactors))
  (if (not (== (Utilities|Array|Length _output_get) 2))
    (Utilities|Time|SetTimerbyEvent (EventDispatchers|CreateEvent :!event Custom|Retry) 1.0)))

(fn ConstructionScript
  (Rendering|Material|SetMaterial (Variables|Default|GetSphere) 0 "/Game/YouTube/Assets/Materials/Instances/Emissive/MI_EmissiveBlack.MI_EmissiveBlack"))