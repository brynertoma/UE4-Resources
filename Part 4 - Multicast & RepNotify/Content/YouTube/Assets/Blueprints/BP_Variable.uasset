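; BP_Variable is an actor made of a middle cylinder and two spheres, with a Relevancy component that appears to visualize its network relevancy range.
; The construction script creates one dynamic instance of MI_EmissiveWhite, tints it with StartingColor and shares it across the three shapes.
; It then sets Relevancy's world scale to twice the square root of NetCullDistanceSquared, matching the diameter of the net cull distance.
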(fn ConstructionScript
  (bind _returnvalue (Rendering|Material|CreateDynamicMaterialInstance "/Game/YouTube/Assets/Materials/Instances/Emissive/MI_EmissiveWhite.MI_EmissiveWhite" "None" :!class /Script/Engine.KismetMaterialLibrary))
  (bind _output_get (Variables|Settings|SetMaterial _returnvalue))
  (Rendering|Material|SetVectorParameterValue _output_get "EmissiveColor" (Variables|Settings|GetStartingColor) :!class /Script/Engine.MaterialInstanceDynamic)
  (Rendering|Material|SetMaterial (Variables|Default|GetCylinderMiddle) 0 (Variables|Settings|GetMaterial))
  (Transformation|SetWorldScale3D (Variables|Default|GetRelevancy) (Math|Conversions|ToVector(Float) (* 2 (Math|Float|Sqrt (Variables|Default|GetNetCullDistanceSquared))))))