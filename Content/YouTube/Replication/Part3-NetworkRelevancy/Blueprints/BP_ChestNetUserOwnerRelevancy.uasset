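; Chest actor for a network relevancy example whose button overlap makes the overlapping actor its owner.
; On authority, it calls CL_GetText to read that player's HUD text, which SR_SetText passes back, relying on ownership for the client-server round trip.
; The RepNotify on Text updates the TextRender.
; The construction script gives the button a dynamic emissive material with configurable color and strength.
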(event OnComponentBeginOverlap(Button)
  (params (OverlappedComponent :type Primitive%20Component%20Object%20Reference) (OtherActor :type Actor%20Object%20Reference) (OtherComp :type Primitive%20Component%20Object%20Reference) (OtherBodyIndex :type Integer) (bFromSweep :type Boolean) (SweepResult :type Hit%20Result%20Structure%20%28by%20ref%29))
  (Actor|SetOwner OtherActor)
  (Networking|SwitchHasAuthority
    (:Authority
      (bind _aspp_player (Utilities|Casting|CastToPP_Player OtherActor))
      (CallFunction|CLGetText _aspp_player))))

(event Custom|SR_SetText
  (params (Value :type Text%20%28by%20ref%29))
  (Variables|Default|SetText Value))

(event Custom|CL_GetText
  (params (Player :type PP%20Player%20Object%20Reference))
  (CallFunction|SRSetText (Class|TextBlock|GetText (Variables|/Game/YouTube/Replication/Part3-NetworkRelevancy/Widgets/W_HUD.W_HUD_C|GetPlayer (Variables|/Game/YouTube/Replication/Part3-NetworkRelevancy/PP_Player.PP_Player_C|GetHUD Player)))))

(fn ConstructionScript
  (|CallParentFunction)
  (bind _returnvalue (Rendering|Material|CreateDynamicMaterialInstance (Variables|Default|GetButton) 0 "/Game/YouTube/Assets/Materials/Instances/Emissive/MI_EmissiveBlack.MI_EmissiveBlack" "None" :!class /Script/Engine.PrimitiveComponent))
  (Rendering|Material|SetVectorParameterValue _returnvalue "EmissiveColor" (Variables|Default|GetEmissiveColor) :!class /Script/Engine.MaterialInstanceDynamic)
  (Rendering|Material|SetScalarParameterValue _returnvalue "EmissiveStrength" (Variables|Default|GetEmissiveStrength) :!class /Script/Engine.MaterialInstanceDynamic))

(fn OnRepText
  (Rendering|Components|TextRender|SetText (Variables|Default|GetTextRender) (Variables|Default|GetText)))