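; A sign actor that displays an emissive title and description and can open an optional web link.
; The construction script sets both texts and gives each a dynamic material instance of M_MasterEmissiveText, with separate colors and a shared strength.
; When a link is set, the Wall blocks the Camera channel, and the LaunchURL event opens that link when called.
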(event Custom|LaunchURL
  (if (Variables|Settings|GetLink?)
    (Utilities|Platform|LaunchURL (Variables|Settings|GetLink))))

(fn ConstructionScript
  (CallFunction|SetText)
  (if (Variables|Settings|GetLink?)
    (Collision|SetCollisionResponsetoChannel (Variables|Default|GetWall) "ECC_Camera" "ECR_Block")))

(fn SetText
  (bind _textdescription (Variables|Default|GetTextDescription))
  (Rendering|Components|TextRender|SetText (Variables|Default|GetTextTitle) (Utilities|Text|ToText(String) (Variables|Settings|GetTitle)))
  (bind _returnvalue (Rendering|Material|CreateDynamicMaterialInstance (Variables|Default|GetTextTitle) 0 "/Game/Assets/Materials/M_MasterEmissiveText.M_MasterEmissiveText" "None" :!class /Script/Engine.PrimitiveComponent))
  (Rendering|Material|SetVectorParameterValue _returnvalue "EmissiveColor" (Variables|Settings|GetEmissiveColor) :!class /Script/Engine.MaterialInstanceDynamic)
  (Rendering|Material|SetScalarParameterValue _returnvalue "EmissiveStrength" (Variables|Settings|GetEmissiveStrength) :!class /Script/Engine.MaterialInstanceDynamic)
  (Rendering|Components|TextRender|SetText _textdescription (Utilities|Text|ToText(String) (Variables|Settings|GetDescription)))
  (bind _returnvalue_2 (Rendering|Material|CreateDynamicMaterialInstance _textdescription 0 "/Game/Assets/Materials/M_MasterEmissiveText.M_MasterEmissiveText" "None" :!class /Script/Engine.PrimitiveComponent))
  (Rendering|Material|SetVectorParameterValue _returnvalue_2 "EmissiveColor" (Variables|Settings|GetEmissiveColor2) :!class /Script/Engine.MaterialInstanceDynamic)
  (Rendering|Material|SetScalarParameterValue _returnvalue_2 "EmissiveStrength" (Variables|Settings|GetEmissiveStrength) :!class /Script/Engine.MaterialInstanceDynamic))