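; BP_Wall is a display fixture that demonstrates a selectable comparison or logic operator on toggleable Boolean inputs, lighting a bulb when the result is true.
; The construction script builds labels, legs, collision spheres and dynamic materials for one, two or three inputs, depending on the Operation enum.
; Toggle maps the passed component to A, B or C by its collision index, flips it and recolours that input.
; LeMagic then evaluates Result and drives the bulb material and point light.
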(event Custom|Toggle
  (params (Component :type Primitive%20Component%20Object%20Reference))
  (Toggles|ToggleBoolean Component)
  (Toggles|ToggleMaterial)
  (CallFunction|LeMagic))

(event EventBeginPlay
  (CallFunction|LeMagic))

(fn ConstructionScript
  (bind _operation (Variables|Settings|GetOperation))
  (Setters|SetText)
  (Setters|SetInputsandCollision)
  (Setters|SetBulbMaterials)
  (Setters|SetInputsMaterials (Variables|Default|GetLegs))
  (if (or (Utilities|Enum|Equal(Enum) _operation "NewEnumerator5") (Utilities|Enum|Equal(Enum) _operation "NewEnumerator14"))
    (Setters|SetInputsMaterials (Variables|Default|GetLegs2)))
  (CallFunction|LeMagic))

(fn LeMagic
  (switch Utilities|FlowControl|Switch|SwitchonE_Operations (Variables|Settings|GetOperation)
    (:NewEnumerator6
      ;[0 0 0 1 50] COMPARISON OPERATORS
      ;;[0 1 0 0.1] EQUAL
      ;; [ A must EQUAL B ]
      (Variables|Other|SetResult (Math|Boolean|Equal(Boolean) (Variables|Other|GetA) (Variables|Other|GetB))))
    (:NewEnumerator7
      ;;[1 0 0 0.1] NOT EQUAL
      ;; [ A must NOT EQUAL B ]
      (Variables|Other|SetResult (Math|Boolean|NotEqual(Boolean) (Variables|Other|GetA) (Variables|Other|GetB))))
    (:NewEnumerator11
      ;;[0 1 0 0.1] GREATER THAN
      ;; [ A is GREATER THAN B]
      (Variables|Other|SetResult (> (Math|Conversions|ToInteger(Boolean) (Variables|Other|GetA)) (Math|Conversions|ToInteger(Boolean) (Variables|Other|GetB)))))
    (:NewEnumerator10
      ;;[1 0 0 0.1] NOT EQUAL
      ;; [ A is LESS THAN B ]
      (Variables|Other|SetResult (< (Math|Conversions|ToInteger(Boolean) (Variables|Other|GetA)) (Math|Conversions|ToInteger(Boolean) (Variables|Other|GetB)))))
    (:NewEnumerator13
      ;;[0 1 0 0.1] GREATER THAN or EQUAL
      ;; [ A is GREATER THAN or EQUAL to B ]
      (Variables|Other|SetResult (>= (Math|Conversions|ToInteger(Boolean) (Variables|Other|GetA)) (Math|Conversions|ToInteger(Boolean) (Variables|Other|GetB)))))
    (:NewEnumerator12
      ;;[1 0 0 0.1] LESS THAN or EQUAL
      ;; [ A is LESS THAN or EQUAL to B ]
      (Variables|Other|SetResult (<= (Math|Conversions|ToInteger(Boolean) (Variables|Other|GetA)) (Math|Conversions|ToInteger(Boolean) (Variables|Other|GetB)))))
    (:NewEnumerator9
      ;[0 0.25 1 0.1] NOT
      ; [ Set the value to the opposite of what it is ]
      (Variables|Other|SetResult (not (Variables|Other|GetA))))
    (:NewEnumerator0
      ;[0 0 0 1 50] LOGICAL OPERATORS
      ;;[0 1 0 0.1] AND
      ;; [ ALL Booleans must be TRUE ]
      (Variables|Other|SetResult (and (Variables|Other|GetA) (Variables|Other|GetB))))
    (:NewEnumerator1
      ;;[0 1 0 0.1] OR
      ;; [ ANY Boolean must be TRUE ]
      (Variables|Other|SetResult (or (Variables|Other|GetA) (Variables|Other|GetB))))
    (:NewEnumerator4
      ;;[1 0 0 0.1] NOR
      ;; [ ALL Booleans must be FALSE ]
      (Variables|Other|SetResult (Math|Boolean|NORBoolean (Variables|Other|GetA) (Variables|Other|GetB))))
    (:NewEnumerator3
      ;;[1 0 0 0.1] NAND
      ;; [ ANY Boolean must be FALSE ]
      (Variables|Other|SetResult (Math|Boolean|NANDBoolean (Variables|Other|GetA) (Variables|Other|GetB))))
    (:NewEnumerator5
      ;;[0 1 0 0.1] XOR - "Exclusive Or"
      ;; [ An ODD # of TRUE Booleans will return TRUE ]
      (Variables|Other|SetResult (Class|KismetMathLibrary|XORBoolean (Class|KismetMathLibrary|XORBoolean (Variables|Other|GetA) (Variables|Other|GetB)) (Variables|Other|GetC))))
    (:NewEnumerator14
      ;;[1 0 0 0.1] XNOR
      ;; [ An EVEN # of TRUE Booleans will return TRUE ]
      (Variables|Other|SetResult (not (Class|KismetMathLibrary|XORBoolean (Class|KismetMathLibrary|XORBoolean (Variables|Other|GetA) (Variables|Other|GetB)) (Variables|Other|GetC))))))
  (Toggles|ToggleBulb))

(fn SetBulbMaterials
  (for (_array_element _array_index) (Rendering|Material|GetMaterials (Variables|Default|GetBooleanFixture))
    (bind _returnvalue (Rendering|Material|CreateDynamicMaterialInstance (Variables|Default|GetBooleanFixture) _array_index _array_element "None" :!class /Script/Engine.PrimitiveComponent))
    (Rendering|Material|SetVectorParameterValue _returnvalue "Color" (Utilities|Select :Index _array_index :Option%200 "(R=0.088542,G=0.088542,B=0.088542,A=1.000000)" :Option%201 "(R=0.023529,G=0.023529,B=0.023529,A=1.000000)" :Option%202 "(R=0.520833,G=0.513161,B=0.490143,A=1.000000)" :Option%203 "(R=0.723958,G=0.596040,B=0.377062,A=1.000000)") :!class /Script/Engine.MaterialInstanceDynamic)
    (if (== _array_index 1)
      (Variables|Other|SetBulbMaterial _returnvalue))))

(fn SetInputsMaterials
  (params (Target :type Mesh%20Component%20Object%20Reference))
  (for (_array_element _array_index) (Rendering|Material|GetMaterials Target)
    (bind _returnvalue (Rendering|Material|CreateDynamicMaterialInstance Target _array_index _array_element "None" :!class /Script/Engine.PrimitiveComponent))
    (Utilities|Array|Add (Variables|Other|GetInputsMaterials) _returnvalue)
    (Rendering|Material|SetVectorParameterValue _returnvalue "Color" (Utilities|Select :Index _array_index :Option%200 "(R=0.000000,G=1.000000,B=0.000000,A=1.000000)" :Option%201 "(R=1.000000,G=0.000000,B=0.000000,A=1.000000)") :!class /Script/Engine.MaterialInstanceDynamic)
    (Rendering|Material|SetScalarParameterValue _returnvalue "Strength" (Utilities|Select :Index _array_index :Option%200 25.0 :Option%201 5e+01) :!class /Script/Engine.MaterialInstanceDynamic)))

(fn SetInputsandCollision
  (bind _operation (Variables|Settings|GetOperation))
  (bind _returnvalue (AddComponent|AddStaticMeshComponent false))
  (bind _output_get (Variables|Default|SetLegs _returnvalue))
  (Components|StaticMesh|SetStaticMesh _output_get (select (Utilities|Enum|Equal(Enum) (Variables|Settings|GetOperation) "NewEnumerator9") "/Game/Assets/Meshes/BooleanFixture_SM_1Leg.BooleanFixture_SM_1Leg" "/Game/Assets/Meshes/BooleanFixture_SM_2Legs.BooleanFixture_SM_2Legs"))
  (bind _returnvalue_2 (AddComponent|AddSphereComponent false (Math|Transform|MakeTransform (Math|Vector|MakeVector 128.5 (Math|Float|SelectFloat 0.0 1e+02 (Utilities|Enum|Equal(Enum) (Variables|Settings|GetOperation) "NewEnumerator9")) -1.5e+02) "0, 0, 0" "0.500000,0.500000,0.500000")))
  (Utilities|Array|Add (Variables|Other|GetCollisions) _returnvalue_2)
  (if (Utilities|Enum|Equal(Enum) (Variables|Settings|GetOperation) "NewEnumerator9")
    (AddComponent|AddTextRenderComponent false)
    (else
      (AddComponent|AddTextRenderComponent false)
      (AddComponent|AddTextRenderComponent false)
      (bind _returnvalue_3 (AddComponent|AddSphereComponent false (Math|Transform|MakeTransform "128.500000,-100.000000,-150.000000" "0, 0, 0" "0.500000,0.500000,0.500000")))
      (Utilities|Array|Add (Variables|Other|GetCollisions) _returnvalue_3)
      (if (or (Utilities|Enum|Equal(Enum) _operation "NewEnumerator5") (Utilities|Enum|Equal(Enum) _operation "NewEnumerator14"))
        (bind _returnvalue_4 (AddComponent|AddStaticMeshComponent false))
        (Variables|Default|SetLegs2 _returnvalue_4)
        (bind _returnvalue_5 (AddComponent|AddSphereComponent false (Math|Transform|MakeTransform "128.500000,0.000000,-150.000000" "0, 0, 0" "0.500000,0.500000,0.500000")))
        (Utilities|Array|Add (Variables|Other|GetCollisions) _returnvalue_5)
        (AddComponent|AddTextRenderComponent false)))))

(fn SetText
  (bind _operation (Variables|Settings|GetOperation))
  (Rendering|Components|TextRender|SetText (Variables|Default|GetTextOperation) (Utilities|Text|ToText(String) (Utilities|String|SelectString "! " (Utilities|String|EnumtoString _operation) (Utilities|Enum|Equal(Enum) _operation "NewEnumerator9"))))
  (bind _returnvalue (Rendering|Material|CreateDynamicMaterialInstance (Variables|Default|GetTextOperation) 0 "/Game/Assets/Materials/M_MasterEmissiveText.M_MasterEmissiveText" "None" :!class /Script/Engine.PrimitiveComponent))
  (Rendering|Material|SetVectorParameterValue _returnvalue "EmissiveColor" (Variables|Settings|GetEmissiveColor) :!class /Script/Engine.MaterialInstanceDynamic)
  (Rendering|Material|SetScalarParameterValue _returnvalue "EmissiveStrength" (Variables|Settings|GetEmissiveStrength) :!class /Script/Engine.MaterialInstanceDynamic)
  (Rendering|Components|TextRender|SetText (Variables|Default|GetTextDescription) (Utilities|Text|ToText(String) (Utilities|Select :Index (Variables|Settings|GetOperation) :NewEnumerator6 "[ A must equal B ]" :NewEnumerator7 "[ A must not equal B]" :NewEnumerator11 "[ A must be greater than B ]" :NewEnumerator10 "[ A must be less than B ]" :NewEnumerator13 "[ A must be greater than or equal to B ]" :NewEnumerator12 "[ A must be less than or equal to B ]" :NewEnumerator9 "" :NewEnumerator0 "[ ALL inputs must be TRUE ]" :NewEnumerator1 "[ ANY input must be TRUE ]" :NewEnumerator4 "[ ALL inputs must be FALSE ]" :NewEnumerator3 "[ ANY input must be FALSE ]" :NewEnumerator5 "[ Any ODD number of TRUEs will return TRUE ]" :NewEnumerator14 "[ Any EVEN number of TRUEs will return TRUE ]"))))

(fn ToggleMaterial
  (Rendering|Material|SetVectorParameterValue (Utilities|Array|Get(acopy) (Variables|Other|GetInputsMaterials) (Variables|Other|GetIndex)) "Color" (Math|Color|SelectColor "(R=0.000000,G=1.000000,B=0.000000,A=1.000000)" "(R=1.000000,G=0.000000,B=0.000000,A=1.000000)" (Utilities|Select :Index (Variables|Other|GetIndex) :Option%200 (Variables|Other|GetA) :Option%201 (Variables|Other|GetB) :Option%202 (Variables|Other|GetC))) :!class /Script/Engine.MaterialInstanceDynamic))

(fn ToggleBulb
  (Rendering|Material|SetVectorParameterValue (Variables|Other|GetBulbMaterial) "Color" (Math|Color|SelectColor "(R=1.000000,G=1.000000,B=1.000000,A=1.000000)" "(R=0.023529,G=0.023529,B=0.023529,A=1.000000)" (Variables|Other|GetResult)) :!class /Script/Engine.MaterialInstanceDynamic)
  (Rendering|Material|SetScalarParameterValue (Variables|Other|GetBulbMaterial) "Strength" (Math|Float|SelectFloat (Math|Float|SelectFloat 5e+02 25.0 (Utilities|Enum|Equal(Enum) (Variables|Settings|GetOperation) "NewEnumerator9")) 1.0 (Variables|Other|GetResult)) :!class /Script/Engine.MaterialInstanceDynamic)
  (Rendering|Components|Light|SetIntensity (Variables|Default|GetPointLight) (Math|Float|SelectFloat (Math|Float|SelectFloat 2.5e+06 1.5e+03 (Utilities|Enum|Equal(Enum) (Variables|Settings|GetOperation) "NewEnumerator9")) 0.0 (Variables|Other|GetResult))))

(fn ToggleBoolean
  (params (InputPin :type Primitive%20Component%20Object%20Reference))
  (bind _output_get (Variables|Other|SetIndex (Utilities|Array|FindItem (Variables|Other|GetCollisions) InputPin)))
  (|SetBy-RefVar (Utilities|Select :Index _output_get :Option%200 (Variables|Other|GetA) :Option%201 (Variables|Other|GetB) :Option%202 (Variables|Other|GetC)) (not (Utilities|Select :Index _output_get :Option%200 (Variables|Other|GetA) :Option%201 (Variables|Other|GetB) :Option%202 (Variables|Other|GetC)))))