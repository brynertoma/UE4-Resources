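; PC_Player is a player controller that owns the player's HUD and relays screen changes to it.
; On BeginPlay, the local controller creates a W_HUD widget and adds it to the viewport.
; SR_ events relay to client-side updates, and CL_ events forward to the HUD through wrapper functions, following a server-to-client naming pattern.
; Each path has INT and ENUM variants for specifying the screen.
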(event Custom|CL_UpdateScreenENUM
  (params (Screen :type E_Screens%20Enum :default "NewEnumerator0"))
  ;[1 1 0 0.25 48] BEGIN PLAY
  ;;[0 0.1559 0.1274 0.25] Update using ENUM
  (PlayerUI|UpdateScreenENUM Screen))

(event Custom|SR_UpdateScreenENUM
  (params (Screen :type E_Screens%20Enum :default "NewEnumerator0"))
  ;[1 1 0 0.25 48] BEGIN PLAY
  ;;[0 0.1559 0.1274 0.25] Update using ENUM
  (CallFunction|CLUpdateScreenENUM Screen))

(event Custom|SR_UpdateScreenINT
  (params (Screen :type Integer))
  ;[1 1 0 0.25 48] BEGIN PLAY
  ;;[0.01298 0.7529 0.4125 0.25] Update using INT
  (CallFunction|CLUpdateScreenINT Screen))

(event Custom|CL_UpdateScreenINT
  (params (Screen :type Integer))
  ;[1 1 0 0.25 48] BEGIN PLAY
  ;;[0.01298 0.7529 0.4125 0.25] Update using INT
  (PlayerUI|UpdateScreenINT Screen))

(event EventBeginPlay
  ;[1 1 0 0.25 48] BEGIN PLAY
  (if (Pawn|IsLocalPlayerController)
    (bind _returnvalue (UserInterface|CreateWidget "/Game/Widgets/W_HUD.W_HUD_C"))
    (bind _output_get (Variables|Default|SetHUD _returnvalue))
    (UserInterface|Viewport|AddtoViewport _output_get 0)))

(fn ConstructionScript)

(fn UpdateScreenINT
  (params (Screen :type Integer))
  (Default|UpdateScreenINT (Variables|Default|GetHUD) Screen))

(fn UpdateScreenENUM
  (params (Screen :type E_Screens%20Enum :default "NewEnumerator0"))
  (Default|UpdateScreenENUM (Variables|Default|GetHUD) Screen))