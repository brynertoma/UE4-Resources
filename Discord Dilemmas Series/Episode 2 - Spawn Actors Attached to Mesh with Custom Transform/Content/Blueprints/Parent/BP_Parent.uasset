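; BP_Parent is a base Blueprint for an object with a mesh that attaches to a socket on a pawn's mesh.
; On BeginPlay it sets its static mesh from GetMesh, which returns nothing here, and applies location and rotation offsets to it.
; Only the authority then performs the attachment, snapping location, rotation and scale to the socket named by the Socket enum.
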(event EventBeginPlay
  (Components|StaticMesh|SetStaticMesh (Variables|Default|GetMesh) (CallFunction|GetMesh))
  (Transformation|SetRelativeLocationAndRotation (Variables|Default|GetMesh) (Variables|Settings|GetLocationOffset) (Variables|Settings|GetRotationOffset) false false)
  (Networking|SwitchHasAuthority
    (:Authority
      (Transformation|AttachComponentToComponent (Variables|/Script/Engine.Character|GetMesh (Variables|Settings|GetPawn)) (Utilities|String|StringToName (Utilities|String|EnumtoString (Variables|Settings|GetSocket))) "SnapToTarget" "SnapToTarget" "SnapToTarget" false))))

(fn ConstructionScript)

(fn GetMesh
  (return 0))