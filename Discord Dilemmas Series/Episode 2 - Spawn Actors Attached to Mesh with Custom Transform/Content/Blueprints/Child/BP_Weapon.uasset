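; BP_Weapon is a child weapon Blueprint that represents either a tier 1 hatchet or knife, chosen by its Variation setting.
; The construction script assigns the matching static mesh through GetMesh.
; BeginPlay selects location and rotation offsets for that variation before calling the parent's BeginPlay, then prints the actor's display name.
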(event EventBeginPlay
  (bind _variation (Variables|Default|GetVariation))
  (Variables|Default|SetLocationOffset (Utilities|Select :Index _variation :Option%200 "0, 0,-10.000000" :Option%201 "0.000000,0.000000,0.000000"))
  (Variables|Default|SetRotationOffset (Utilities|Select :Index _variation :Option%200 "0,180.000000, 0" :Option%201 "180.000000,0.000000,0.000000"))
  (|CallParentFunction)
  (Development|PrintString (Utilities|GetDisplayName self) true true "(R=1.000000,G=0.000000,B=0.000000,A=1.000000)" 1e+01))

(fn ConstructionScript
  (Components|StaticMesh|SetStaticMesh (Variables|Character|GetMesh) (CallFunction|GetMesh)))

(fn GetMesh
  (return (Utilities|Select :Index (Variables|Default|GetVariation) :Option%200 "/Game/Mesh/SM_T1Hatchet.SM_T1Hatchet" :Option%201 "/Game/Mesh/SM_T1Knife.SM_T1Knife")))