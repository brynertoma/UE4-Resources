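; Example game mode that runs a simple before, during and end match flow and switches each player's HUD screen to match.
; PostLogin caches cast PC_Player controllers and starts the match when the added index equals MaxPlayers; otherwise a BeginPlay timer starts it.
; Starting sets a short timer that ends the match.
; Screen changes loop over the cached controllers, demonstrating both an enum and an integer-index version of the update call.
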(event Custom|StartGame
  ;[1 1 0 0.25 48] BEGIN PLAY
  ;;[1 1 0 0.25] After 3 seconds, start the game if it hasn't already been started by max player count being hit.
  ;;
  ;; This example is using the INT version of the update widgets function. Based on the array we created in W_HUD:
  ;;
  ;; 0 = W_GameBefore
  ;; 1 = W_GameDuring
  ;; 2 = W_GameEnd
  (if (not (Variables|Default|GetStarted?))
    (Variables|Default|SetStarted? true)
    (PlayerUI|UpdatePlayerWidgetsINT 1)
    (CallFunction|StartEndGameTimer)))

(event Custom|StartEndGameTimer
  ;[1 1 0 0.25 48] BEGIN PLAY
  ;;[1 1 0 0.25] Start the end timer then update the player UI to end game when it goes off.
  (Utilities|Time|SetTimerbyEvent (delegate Custom|EndGame) 3.0))

(event Custom|EndGame
  ;[1 1 0 0.25 48] BEGIN PLAY
  ;;[1 1 0 0.25] Start the end timer then update the player UI to end game when it goes off.
  (Variables|Default|SetStarted? false)
  (PlayerUI|UpdatePlayerWidgetsENUM "NewEnumerator2"))

(event EventPostLogin
  (params (NewPlayer :type Player%20Controller%20Object%20Reference))
  ;[1 1 0 0.25 48] BEGIN PLAY
  ;;[1 1 0 0.25] We want to capture player controllers as they join (we cast them here so that we don't have to cast later - especially if we iterate through the controllers over and over again).
  ;;
  ;; This example is using the ENUM version of the update widgets function.
  (if (not (Variables|Default|GetStarted?))
    (bind _aspc_player (Utilities|Casting|CastToPC_Player NewPlayer))
    (bind _returnvalue (Utilities|Array|Add (Variables|Default|GetControllers) _aspc_player))
    (if (== _returnvalue (Variables|Default|GetMaxPlayers))
      (PlayerUI|UpdatePlayerWidgetsENUM "NewEnumerator1")
      (Variables|Default|SetStarted? true)
      (CallFunction|StartEndGameTimer))))

(event EventBeginPlay
  ;[1 1 0 0.25 48] BEGIN PLAY
  ;;[1 1 0 0.25] After 3 seconds, start the game if it hasn't already been started by max player count being hit.
  ;;
  ;; This example is using the INT version of the update widgets function. Based on the array we created in W_HUD:
  ;;
  ;; 0 = W_GameBefore
  ;; 1 = W_GameDuring
  ;; 2 = W_GameEnd
  (Utilities|Time|SetTimerbyEvent (delegate Custom|StartGame) 3.0))

(fn ConstructionScript)

(fn UpdatePlayerWidgetsINT
  (params (Screen :type Integer))
  (for _array_element (Variables|Default|GetControllers)
    (Default|SRUpdateScreenINT _array_element Screen)))

(fn UpdatePlayerWidgetsENUM
  (params (Screen :type E_Screens%20Enum :default "NewEnumerator0"))
  (for _array_element (Variables|Default|GetControllers)
    (Default|CLUpdateScreenENUM _array_element Screen)))