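; BP_VariableNone is a replication demo actor that displays a changing random number on a TextRender component.
; On BeginPlay, only the authority starts a looping one-second timer bound to the Update event.
; Update stores a random float in Variable and writes it straight to the text, with no RepNotify or multicast to update the text on clients.
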(event Custom|Update
  (bind _output_get (Variables|Default|SetVariable (Math|Random|RandomFloatinRange 0.0 1e+04)))
  (Rendering|Components|TextRender|SetText (Variables|Default|GetTextRender) (Utilities|Text|ToText(Float) _output_get "HalfToEven")))

(event EventBeginPlay
  (|CallParentFunction)
  (Networking|SwitchHasAuthority
    (:Authority
      (Utilities|Time|SetTimerbyEvent (delegate Custom|Update) 1.0 true))))

(fn ConstructionScript
  (|CallParentFunction))