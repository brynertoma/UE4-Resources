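; Replication demo actor: a sphere that bobs up and down, with a RelevancySphere visualizing its network cull distance.
; On BeginPlay, only the authority runs the Move timeline at half speed, lerping the sphere along its up vector and back, looping through a FlipFlop on Finished.
; The construction script sizes RelevancySphere from NetCullDistanceSquared.
; An unconnected loop for destroying non-NetLoadOnClient actors on clients never runs.
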(event EventBeginPlay
  (bind _sphere (Variables|Default|GetSphere))
  (Networking|SwitchHasAuthority
    (:Authority
      (bind _output_get (Variables|Default|SetStart (Transformation|GetWorldLocation _sphere)))
      (Variables|Default|SetEnd (+ _output_get (* (Math|Vector|GetUpVector _sphere) 200)))
      (Components|Timeline|SetPlayRate (Variables|Default|GetMove) 0.5)
      (Utilities|FlowControl|FlipFlop :!label _label
        (:A
          (bind _alpha (Timeline|Move PlayFromStart)
            (:Update
              (Transformation|SetWorldLocation (Variables|Default|GetSphere) (Math|Vector|Lerp(Vector) (Variables|Default|GetStart) (Variables|Default|GetEnd) _alpha) false false))
            (:Finished
              (goto _label))))
        (:B
          (Timeline|Move ReverseFromEnd))))))

(fn ConstructionScript
  (Transformation|SetWorldScale3D (Variables|Default|GetRelevancySphere) (Math|Conversions|ToVector(Float) (* 2 (Math|Float|Sqrt (Variables|Default|GetNetCullDistanceSquared))))))